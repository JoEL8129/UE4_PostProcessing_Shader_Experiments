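; Player controller for an RTS-style game that creates the main HUD and manages a set of selected units.
; On start it locks the mouse in game-and-UI input mode and adds the HUD widget to the viewport.
; Add and remove functions maintain the selection array and toggle each unit's selected state.
; Right-click traces under the cursor and writes the hit location to each selected unit's Blackboard TargetVector.
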(event EventBeginPlay
  (Utilities|FlowControl|Sequence
    (:then_0
      (Input|SetInputModeGameandUI self 0 "LockAlways" false))
    (:then_1
      (bind _returnvalue (UserInterface|CreateWidget "/Game/_Main/BLUEPRINTS/Widgets/UI_HUD.UI_HUD_C"))
      (bind _output_get (Variables|Default|SetMainUIWidget _returnvalue))
      (UserInterface|Viewport|AddtoViewport _output_get 0))))

(event Input|MouseEvents|RightMouseButton
  (params (Key :type Key%20Structure :default "None"))
  (bind (_hitresult _returnvalue) (Game|Player|GetHitResultUnderCursorbyChannel "TraceTypeQuery1" true))
  ;[1 1 1] RightMouse
  (:Pressed
    (if (CallFunction|CheckifSomethingSelected)
      (if _returnvalue
        (for _array_element (Variables|Default|GetUnitSelection)
          (AI|Components|Blackboard|SetValueasVector (AI|GetBlackboard _array_element) (Utilities|Name|MakeLiteralName "TargetVector") (.location _hitresult)))))))

(fn ConstructionScript)

(fn AddUnittoSelection
  (params (Unit :type Unit%20Base%20Object%20Reference))
  (Utilities|Array|AddUnique (Variables|Default|GetUnitSelection) Unit)
  (Default|IsSelected Unit true))

(fn RemoveUnitfromSelection
  (params (Unit :type Unit%20Base%20Object%20Reference))
  (Utilities|Array|RemoveItem (Variables|Default|GetUnitSelection) Unit)
  (Default|IsSelected Unit false))

(fn CheckifSomethingSelected
  (return (!= (Utilities|Array|Length (Variables|Default|GetUnitSelection)) 0)))