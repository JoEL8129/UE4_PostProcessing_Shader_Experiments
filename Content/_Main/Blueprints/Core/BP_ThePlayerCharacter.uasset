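; Player character for cursor-aimed play: spawns its own RTSCamera, yaws toward a mouse trace every tick, and moves on the ground plane.
; Space jumps, or with WASD held performs a two-stage launch dash, varied by Shift, with a double charge before cooldown.
; Left click fires projectiles at a forward trace's hit point, or straight ahead.
; Damage reduces Health, and death destroys character and camera; other keys control the camera.
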(event Custom|Death
  (Actor|DestroyActor (Variables|Default|GetMainCam))
  (Actor|DestroyActor))

(event Custom|GotDamaged
  (params (DamagedActor :type Actor%20Object%20Reference) (Damage :type Float%20%28single-precision%29) (DamageType :type Damage%20Type%20Object%20Reference) (InstigatedBy :type Controller%20Object%20Reference) (DamageCauser :type Actor%20Object%20Reference))
  (CallFunction|ReceiveDamage Damage)
  (CallFunction|CheckHealth))

(event EventBeginPlay
  (bind _returnvalue (Game|SpawnActorfromClass "/Game/_Main/Blueprints/Actors/Camera/RTSCamera.RTSCamera_C" (Math|Transform|MakeTransform (Transformation|GetActorLocation) "0, 0, 0" "1,1,1") "Undefined" 0 0))
  (Variables|Default|SetMainCam _returnvalue)
  (bind _asbp_the_player_controller (Utilities|Casting|CastToBP_ThePlayerController (Game|GetPlayerController 0)))
  (Variables|Default|SetPlayerControllerREF _asbp_the_player_controller)
  (EventDispatchers|BindEventtoOnTakeAnyDamage (delegate Custom|GotDamaged)))

(event EventTick
  (params (DeltaSeconds :type Float%20%28single-precision%29))
  (CallFunction|LookatCursor))

(event Input|AxisEvents|InputAxisMoveForward
  (params (AxisValue :type Float%20%28single-precision%29))
  (Pawn|Input|AddMovementInput (Math|Vector|GetForwardVector (Math|Rotator|MakeRotator 0.0 0.0 (.Yaw (Math|Rotator|BreakRotator (select (Variables|Default|GetUseRotationForMovement?) (Transformation|GetActorRotation) "0, 0, 0"))))) AxisValue false))

(event Input|AxisEvents|InputAxisMoveRight
  (params (AxisValue :type Float%20%28single-precision%29))
  (Pawn|Input|AddMovementInput (Math|Vector|GetRightVector (Math|Rotator|MakeRotator 0.0 0.0 (.Yaw (Math|Rotator|BreakRotator (select (Variables|Default|GetUseRotationForMovement?) (Transformation|GetActorRotation) "0, 0, 0"))))) AxisValue false))

(event Input|KeyboardEvents|SpaceBar
  (params (Key :type Key%20Structure :default "None"))
  (bind (_wasd _shift) (CallFunction|AreWASDdown?))
  (:Pressed
    (if _wasd
      (if _shift
        (Variables|Default|SetDashHeight 3e+02)
        (Variables|Default|SetDashDistance 8e+02)
        (else
          (Variables|Default|SetDashHeight 8e+02)
          (Variables|Default|SetDashDistance 1e+02)))
      (Utilities|FlowControl|DoOnce false :!label _label
        (:Completed
          (Character|LaunchCharacter (Math|Vector|MakeVector 0.0 0.0 (Variables|Default|GetDashHeight)) false false)
          (Utilities|FlowControl|Delay 0.1)
          (Character|LaunchCharacter (* (Math|Vector|GetForwardVector (Transformation|GetActorRotation)) (Variables|Default|GetDashDistance)) false false)
          (Animation|PlayAnimMontage "/Game/_Main/Blueprints/Animation/NewAnimMontage.NewAnimMontage" 1.0 "None")
          (if (Variables|Default|GetFirstDash?)
            (Variables|Default|SetFirstDash? false)
            (goto _label Reset)
            (else
              (Utilities|FlowControl|Delay (Variables|Default|GetDashCooldown))
              (Variables|Default|SetFirstDash? true)
              (goto _label Reset)))))
      (else
        (Character|Jump))))
  (:Released
    (if (not _wasd)
      (Character|StopJumping))))

(event Input|KeyboardEvents|F
  (params (Key :type Key%20Structure :default "None"))
  (:Pressed
    (Transformation|SetActorLocation (Variables|Default|GetMainCam) (Transformation|GetActorLocation) false false)))

(event Input|KeyboardEvents|E
  (params (Key :type Key%20Structure :default "None"))
  (:Pressed
    (Development|PrintString (Utilities|String|ToString(Vector) "0, 0, 0"))))

(event Input|MouseEvents|MouseWheelUp
  (params (Key :type Key%20Structure :default "None"))
  (:Pressed
    (Default|Zoomin (Variables|Default|GetMainCam))))

(event Input|MouseEvents|MouseWheelDown
  (params (Key :type Key%20Structure :default "None"))
  (:Pressed
    (Default|ZoomOut (Variables|Default|GetMainCam))))

(event Input|MouseEvents|LeftMouseButton
  (params (Key :type Key%20Structure :default "None"))
  (bind _self self)
  (bind _projectilespawn (Variables|Default|GetProjectileSpawn))
  (bind _projectilespawn_2 (Variables|Default|GetProjectileSpawn))
  (bind _returnvalue (Transformation|GetWorldLocation _projectilespawn))
  (bind _returnvalue_2 (Transformation|GetWorldRotation _projectilespawn))
  (bind _returnvalue_3 (Transformation|GetWorldTransform _projectilespawn_2))
  (bind _location (Math|Transform|BreakTransform _returnvalue_3))
  (:Pressed
    (bind (_outhit _returnvalue_4) (Collision|LineTraceByChannel _returnvalue (+ (* (Math|Vector|GetForwardVector _returnvalue_2) 5e+03) _returnvalue) "TraceTypeQuery1" false 0 "None"))
    (if _returnvalue_4
      (Game|SpawnActorfromClass "/Game/_Main/Blueprints/Actors/Projectile.Projectile_C" (Math|Transform|MakeTransform _location (Math|Rotator|FindLookatRotation _location (.Location (Collision|BreakHitResult _outhit)))) "AlwaysSpawn" 0 _self)
      (else
        (Game|SpawnActorfromClass "/Game/_Main/Blueprints/Actors/Projectile.Projectile_C" (Math|Transform|MakeTransform _location _returnvalue_2) "AlwaysSpawn" 0 _self)))))

(event Input|KeyboardEvents|NumPadOne
  (params (Key :type Key%20Structure :default "None"))
  (:Pressed
    (Default|CamSwitch (Variables|Default|GetMainCam))))

(fn ConstructionScript)

(fn LookatCursor
  (bind _playercontrollerref (Variables|Default|GetPlayerControllerREF))
  (bind (_worldlocation _worlddirection) (Game|Player|ConvertMouseLocationToWorldSpace _playercontrollerref))
  (bind _outhit (Collision|LineTraceByChannel _worldlocation (+ _worldlocation (* _worlddirection (+ (Variables|/Game/_Main/Blueprints/Actors/Camera/RTSCamera.RTSCamera_C|GetTarget%20Arm%20Length (Variables|Default|GetMainCam)) 5e+03))) "TraceTypeQuery1" false 0 "None"))
  (bind _output_get (Variables|Default|SetDirection (.location _outhit)))
  (Transformation|SetActorRotation (Math|Rotator|MakeRotator (.roll (Math|Rotator|FindLookatRotation (Transformation|GetActorLocation) _output_get)) 0.0 (.yaw (Math|Rotator|FindLookatRotation (Transformation|GetActorLocation) _output_get)))))

(fn CheckHealth
  (if (<= (Variables|Attributes|GetHealth) 0.0)
    (CallFunction|Death)))

(fn ReceiveDamage
  (params (Damage :type Float%20%28single-precision%29))
  (Variables|Attributes|SetHealth (- (Variables|Attributes|GetHealth) Damage)))

(fn AreWASDdown?
  (bind _returnvalue (Game|GetPlayerController 0))
  (return (Math|Boolean|ORBoolean (Game|Player|IsInputKeyDown _returnvalue "W") (Game|Player|IsInputKeyDown _returnvalue "A") (Game|Player|IsInputKeyDown _returnvalue "S") (Game|Player|IsInputKeyDown _returnvalue "D")) (Game|Player|IsInputKeyDown _returnvalue "LeftShift")))