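; UnitBase is a base actor for player-selectable units.
; It caches the BP_ThePlayerController on BeginPlay, then on click adds itself to that controller's selection with the left button or removes itself with any other, updating its selected flag.
; A separate IsSelected event shows or hides the selection decal, while IsMoved receives a target position but has no logic here.
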(event Custom|IsSelected
  (params (IsSelected :type Boolean))
  (Rendering|SetVisibility (Variables|Default|GetDecal) IsSelected false))

(event Custom|IsMoved
  (params (TargetPosition :type Vector)))

(event EventBeginPlay
  (bind _asbp_the_player_controller (Utilities|Casting|CastToBP_ThePlayerController (Game|GetPlayerController 0)))
  (Variables|Default|SetPlayerControllerRef _asbp_the_player_controller))

(event Collision|EventActorBeginOverlap
  (params (OtherActor :type Actor%20Object%20Reference)))

(event EventTick
  (params (DeltaSeconds :type Float%20%28single-precision%29)))

(event MouseInput|EventActorOnClicked
  (params (ButtonPressed :type Key%20Structure :default "None"))
  (bind _playercontrollerref (Variables|Default|GetPlayerControllerRef))
  (if (== ButtonPressed "LeftMouseButton")
    (Default|AddUnittoSelection _playercontrollerref self)
    (Variables|Default|SetUnitIsSelected true)
    (else
      (Default|RemoveUnitfromSelection _playercontrollerref self)
      (Variables|Default|SetUnitIsSelected false))))

(fn ConstructionScript)