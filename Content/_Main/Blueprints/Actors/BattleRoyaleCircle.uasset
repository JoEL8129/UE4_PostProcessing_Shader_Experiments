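; Battle royale safe-zone actor that shrinks and damages a player who leaves its sphere collider.
; GettingSmaller and NotGettingSmaller start and stop a looping timer that reduces Size, clamped at zero, and rescales the whole actor.
; Exiting starts a repeating damage timer on the stored player.
; Only the last player to exit is tracked, and any player entering clears the timer.
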(event OnComponentBeginOverlap(SphereCollider)
  (params (OverlappedComponent :type Primitive%20Component%20Object%20Reference) (OtherActor :type Actor%20Object%20Reference) (OtherComp :type Primitive%20Component%20Object%20Reference) (OtherBodyIndex :type Integer) (bFromSweep :type Boolean) (SweepResult :type Hit%20Result%20Structure%20%28by%20ref%29))
  (Utilities|Casting|CastToBP_ThePlayerCharacter OtherActor)
  (Utilities|Time|ClearTimerbyFunctionName 0 "ApplyingDamage"))

(event OnComponentEndOverlap(SphereCollider)
  (params (OverlappedComponent :type Primitive%20Component%20Object%20Reference) (OtherActor :type Actor%20Object%20Reference) (OtherComp :type Primitive%20Component%20Object%20Reference) (OtherBodyIndex :type Integer))
  (bind _asbp_the_player_character (Utilities|Casting|CastToBP_ThePlayerCharacter OtherActor))
  (Variables|Default|SetCircle%20Exiting%20Player _asbp_the_player_character)
  (Utilities|Time|SetTimerbyFunctionName 0 "ApplyingDamage" 1.0 true))

(event Custom|GettingSmaller
  (Utilities|Time|SetTimerbyFunctionName 0 "ReduceSize" 0.05 true))

(event Custom|NotGettingSmaller
  (Utilities|Time|ClearTimerbyFunctionName 0 "ReduceSize"))

(event EventBeginPlay
  (bind _size (Variables|Default|GetSize))
  (Transformation|SetActorScale3D (Math|Vector|MakeVector _size _size _size)))

(event EventTick
  (params (DeltaSeconds :type Float%20%28single-precision%29)))

(fn ConstructionScript)

(fn ReduceSize
  (bind _output_get (Variables|Default|SetSize (Math|Float|Clamp(Float) (- (Variables|Default|GetSize) (Variables|Default|GetSize%20Decrease%20Value)) 0.0 (Variables|Default|GetSize))))
  (Transformation|SetActorScale3D (Math|Vector|MakeVector _output_get _output_get _output_get)))

(fn ApplyingDamage
  (Utilities|IsValid (Variables|Default|GetCircle%20Exiting%20Player)
    (:Is%20Valid
      (Game|Damage|ApplyDamage (Variables|Default|GetCircle%20Exiting%20Player) (Variables|Default|GetDamage) 0 0))
    (:Is%20Not%20Valid
      (Variables|Default|SetCircle%20Exiting%20Player 0))))